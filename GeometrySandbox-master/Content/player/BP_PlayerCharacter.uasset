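; Player character Blueprint that lets the player pick up and drop actors with the mouth.
; Each Tick, a short Visibility trace from the camera stores the hit actor in AHitActor; both branches of the MyInventoryActor class check store it alike.
; GrabUngrabInv toggles GrabActor, attaching that actor to the mesh's mouthSocket or detaching the first attached actor, keeping world transforms.
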(event EventBeginPlay)

(event Collision|EventActorBeginOverlap
  (params (OtherActor :type Actor%20Object%20Reference)))

(event EventTick
  (params (DeltaSeconds :type Float%20%28single-precision%29))
  (bind _cameracomponent (Variables|CameraActor|GetCameraComponent))
  (bind _returnvalue (Transformation|GetWorldLocation _cameracomponent))
  ;[1 1 1] LneTraceByChannel and get current Actor
  (bind _outhit (Collision|LineTraceByChannel _returnvalue (+ (* (Math|Vector|GetForwardVector _cameracomponent) 2e+02) _returnvalue) "TraceTypeQuery1" false 0 "None"))
  (if (== (Utilities|GetClass (.HitActor (Collision|BreakHitResult _outhit))) "/Game/player/MyInventoryActor.MyInventoryActor_C")
    (Variables|Default|SetAHitActor (.HitActor (Collision|BreakHitResult _outhit)))
    (else
      (Variables|Default|SetAHitActor (.HitActor (Collision|BreakHitResult _outhit))))))

(event Input|ActionEvents|InputActionGrabUngrabInv
  (params (Key :type Key%20Structure :default "None"))
  (bind _ahitactor (Variables|Default|GetAHitActor))
  (:Pressed
    ;[1 1 1] GrabUngrub Inventory event
    (if (Variables|Default|GetbGrabActor)
      (Transformation|DetachFromComponent (Variables|/Script/Engine.Actor|GetRootComponent (Utilities|Array|Get(acopy) (Actor|GetAttachedActors true))) "KeepWorld" "KeepWorld" "KeepWorld" true)
      (Variables|Default|SetbGrabActor false)
      (else
        (Utilities|IsValid _ahitactor
          (:Is%20Valid
            (Transformation|AttachComponentToComponent _ahitactor (Variables|Character|GetMesh) "mouthSocket" "KeepWorld" "KeepWorld" "KeepWorld" false)
            (Variables|Default|SetbGrabActor true)))))))

(fn ConstructionScript)