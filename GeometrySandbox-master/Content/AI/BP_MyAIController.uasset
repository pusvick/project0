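; AI controller that makes the AI character follow the player, or flee when the player is holding a grabbed actor nearby.
; BeginPlay caches the first player and AI character found in the level, then runs BP_BehaviorTree.
; Each Tick writes the blackboard Vector: an offset player location for following, or a doubled player-to-AI difference (not world-relative) for fleeing.
; Fleeing also sets rotation to a negated look-at yaw; a grab out of range leaves the Vector unchanged.
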(event EventBeginPlay
  ;[1 1 1] BeginPlay
  ;;[1 1 1] Get player
  (bind _outactors (Actor|GetAllActorsOfClass "/Game/player/BP_PlayerCharacter.BP_PlayerCharacter_C"))
  (Variables|Default|Setplayer (Utilities|Array|Get(acopy) _outactors))
  ;;[1 1 1] Get AI Actor
  (bind _outactors_2 (Actor|GetAllActorsOfClass "/Script/GeometrySandbox.MyAICharacter"))
  (Variables|Default|SetAI (Utilities|Array|Get(acopy) _outactors_2))
  (AI|RunBehaviorTree "/Game/AI/BP_BehaviorTree.BP_BehaviorTree"))

(event EventTick
  (params (DeltaSeconds :type Float%20%28single-precision%29))
  ;[1 1 1] Check Grab Inventory
  (if (Variables|/Script/GeometrySandbox.PlayerCharacter|GetbGrabActor (Variables|Default|Getplayer))
    ;[1 1 1] Check distance between AI and Player
    (if (< (Transformation|GetDistanceTo (Variables|Default|GetAI) (Variables|Default|Getplayer)) 5e+02)
      ;[1 1 1] Run away from player
      (AI|Components|Blackboard|SetValueasVector (AI|GetBlackboard 0) (Variables|Default|GetVector) (* (- (Transformation|GetActorLocation (Variables|Default|GetAI)) (Transformation|GetActorLocation (Variables|Default|Getplayer))) 2))
      ;[1 1 1] Set current rotation
      (Transformation|SetActorRotation (Variables|Default|GetAI) (Math|Rotator|MakeRotator 0.0 0.0 (.Yaw (Math|Rotator|BreakRotator (* (Math|Rotator|FindLookatRotation (Transformation|GetActorLocation (Variables|Default|GetAI)) (Transformation|GetActorLocation (Game|GetPlayerCharacter 0))) -1))))))
    (else
      ;[1 1 1] Follow player
      (AI|Components|Blackboard|SetValueasVector (AI|GetBlackboard 0) (Variables|Default|GetVector) (- (Transformation|GetActorLocation (Variables|Default|Getplayer)) "150.000000,150.000000,150.000000")))))

(fn ConstructionScript)